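; Core HUD that builds the menu screens (main menu, achievements, collection, pack opening, shop) and switches between them.
; On BeginPlay it finds tagged CameraActors, passes each widget its camera, with the shop sharing the index camera, and shows the main menu with mouse input.
; The other menus are preloaded hidden in the viewport.
; ActivateMenu records the previous menu, collapses it, switches camera through PC_Core_BP and reveals the new one.
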(event EventBeginPlay
  (CallFunction|MenuCameraSetup)
  (CallFunction|WidgetSetup))

(fn ConstructionScript)

(fn WidgetSetup
  (bind _returnvalue (Game|Player|GetOwningPlayerController))
  (Utilities|FlowControl|Sequence
    (:then_0
      ;[1 1 1] Parent Widget
      (UserInterface|CreateWidget "/Game/Blueprints/Widgets/_PARENT_UW._PARENT_UW_C" _returnvalue 0)
      ;[1 1 1] Main Menu, Primary Widget
      (bind _returnvalue_2 (UserInterface|CreateWidget "/Game/Blueprints/Widgets/MainMenu_WD.MainMenu_WD_C" _returnvalue (Variables|Default|GetIndexCam)))
      (bind _output_get (Variables|Default|SetMainMenuWD _returnvalue_2))
      (UserInterface|Viewport|AddtoViewport _output_get 0)
      ;[1 1 1] Defaults
      (Variables|/Script/Engine.PlayerController|SetbShowMouseCursor _returnvalue true)
      (Input|SetInputModeGameandUI _returnvalue _output_get "DoNotLock" false false))
    (:then_1
      ;[1 1 1] Loading Widgets to Collapse
      (bind _returnvalue_3 (UserInterface|CreateWidget "/Game/Blueprints/Widgets/Achievements_WD.Achievements_WD_C" _returnvalue (Variables|Default|GetAchievementsCam)))
      (bind _output_get_2 (Variables|Default|SetAchievementsWD _returnvalue_3))
      (Utilities|Array|Add (Variables|Default|GetWidgetsToCollapseList) _output_get_2)
      (bind _returnvalue_4 (UserInterface|CreateWidget "/Game/Blueprints/Widgets/Collection_WD.Collection_WD_C" _returnvalue (Variables|Default|GetCollectionCam)))
      (bind _output_get_3 (Variables|Default|SetCollectionWD _returnvalue_4))
      (Utilities|Array|Add (Variables|Default|GetWidgetsToCollapseList) _output_get_3)
      (bind _returnvalue_5 (UserInterface|CreateWidget "/Game/Blueprints/Widgets/OpenPacks_WD.OpenPacks_WD_C" _returnvalue (Variables|Default|GetOpenPacksCam)))
      (bind _output_get_4 (Variables|Default|SetOpenPacksWD _returnvalue_5))
      (Utilities|Array|Add (Variables|Default|GetWidgetsToCollapseList) _output_get_4)
      (bind _returnvalue_6 (UserInterface|CreateWidget "/Game/Blueprints/Widgets/Shop_WD.Shop_WD_C" _returnvalue (Variables|Default|GetIndexCam)))
      (bind _output_get_5 (Variables|Default|SetShopWD _returnvalue_6))
      (Utilities|Array|Add (Variables|Default|GetWidgetsToCollapseList) _output_get_5))
    (:then_2
      ;[1 1 1] Add to viewport, collapse, remove from list
      (for _array_element (Variables|Default|GetWidgetsToCollapseList)
        (UserInterface|Viewport|AddtoViewport _array_element 0)
        (Widget|SetVisibility _array_element "Hidden"))
      (Utilities|Array|Clear (Variables|Default|GetWidgetsToCollapseList)))))

(fn ActivateMenu
  (params (PreviousMenu :type PARENT%20UW%20Object%20Reference) (NewActiveMenu :type PARENT%20UW%20Object%20Reference) (New%20Active%20Cam :type Camera%20Actor%20Object%20Reference))
  (Utilities|FlowControl|Sequence
    (:then_0
      (Variables|/Game/Blueprints/Widgets/_PARENT_UW._PARENT_UW_C|SetLastMenu NewActiveMenu PreviousMenu)
      (Widget|SetVisibility PreviousMenu "Collapsed"))
    (:then_1
      (bind _aspc_core_bp (Utilities|Casting|CastToPC_Core_BP (Game|Player|GetOwningPlayerController)))
      (Default|ChangeCameras _aspc_core_bp New%20Active%20Cam))
    (:then_2
      (Widget|SetVisibility NewActiveMenu "Visible"))))

(fn MenuCameraSetup
  (Utilities|FlowControl|Sequence
    (:then_0
      (bind _outactors (Actor|GetAllActorsOfClasswithTag "/Script/Engine.CameraActor" "IndexCam"))
      (Variables|Default|SetIndexCam (Utilities|Array|Get(acopy) _outactors)))
    (:then_1
      (bind _outactors_2 (Actor|GetAllActorsOfClasswithTag "/Script/Engine.CameraActor" "AchievementsCam"))
      (Variables|Default|SetAchievementsCam (Utilities|Array|Get(acopy) _outactors_2)))
    (:then_2
      (bind _outactors_3 (Actor|GetAllActorsOfClasswithTag "/Script/Engine.CameraActor" "CollectionCam"))
      (Variables|Default|SetCollectionCam (Utilities|Array|Get(acopy) _outactors_3)))
    (:then_3
      (bind _outactors_4 (Actor|GetAllActorsOfClasswithTag "/Script/Engine.CameraActor" "OpenPacksCam"))
      (Variables|Default|SetOpenPacksCam (Utilities|Array|Get(acopy) _outactors_4)))))